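; PC_WidgetTest is a player controller that, judging by its name, is for testing the session lobby UI.
; On BeginPlay it creates the UMG_SessionLobyy widget, adds it to the viewport, focuses it in Game and UI input mode and shows the mouse cursor.
; Disconnected leftovers hold a UI-only input alternative and a loop that would fill the session list's scroll box with UMG_SessionLine rows.
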(event EventBeginPlay
  (bind _returnvalue (UserInterface|CreateWidget "/Game/Blueprints/Widget/UMG_SessionLobyy.UMG_SessionLobyy_C" self))
  (UserInterface|Viewport|AddtoViewport _returnvalue 0)
  (Variables|Default|SetNewVar_0 0)
  (Input|SetInputModeGameandUI self _returnvalue "DoNotLock" false)
  (Variables|Default|SetbShowMouseCursor true))

(event EventTick
  (params (DeltaSeconds :type Float%20%28single-precision%29)))

(fn ConstructionScript)