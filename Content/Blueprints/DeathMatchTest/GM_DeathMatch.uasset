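; Deathmatch game mode that registers players, spawns their spiders, tracks kills and deaths, and ends the match at a win score.
; PostLogin indexes each PC_DeathMatch in an array, later looped to push player list, scoreboard and game-end events.
; Spawn orders unpossess any current pawn and possess a new BasicSpider at a player start.
; Kill reports trigger delayed scoreboard refreshes or game end, which destroys sessions after a pause and opens MainMap.
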(event Custom|RecieveSpawnOrder
  (params (PlayerController :type Player%20Controller%20Object%20Reference) (UserFreeSet :type User%20Free%20Set%20Structure))
  (Utilities|IsValid (Pawn|GetControlledPawn PlayerController)
    (:Is%20Valid
      (Pawn|UnPossess PlayerController))
    (:Is%20Not%20Valid
      _))
  (bind _aspc_death_match (Utilities|Casting|CastToPC_DeathMatch PlayerController))
  (bind _returnvalue (Game|SpawnActorfromClass "/Game/Blueprints/DeathMatchTest/BasicSpider.BasicSpider_C" (Math|Transform|MakeTransform (.location (Transformation|GetActorTransform (Class|GameModeBase|FindPlayerStart _aspc_death_match))) (.rotation (Transformation|GetActorTransform (Class|GameModeBase|FindPlayerStart _aspc_death_match))) "1,1,1") "AdjustIfPossibleButAlwaysSpawn" _aspc_death_match 0))
  (Pawn|Possess _aspc_death_match _returnvalue))

(event Custom|OrderPlayerListUpdate
  (for _array_element (Variables|Default|GetPlayerControllerArray)
    (Default|OnResetPlayerList _array_element)))

(event Custom|OrderPlayerScoreUpdate
  (for _array_element (Variables|Default|GetPlayerControllerArray)
    (Default|OnRearrangeScoreBoard _array_element)))

(event Custom|GetKillReport
  (params (KillerPlayerState :type PS%20Death%20Match%20Object%20Reference) (DeadPlayerState :type PS%20Death%20Match%20Object%20Reference))
  (bind _output_get (Variables|/Game/Blueprints/DeathMatchTest/PS_DeathMatch.PS_DeathMatch_C|SetKill KillerPlayerState (+ (Variables|/Game/Blueprints/DeathMatchTest/PS_DeathMatch.PS_DeathMatch_C|GetKill KillerPlayerState) 1)))
  (Variables|/Game/Blueprints/DeathMatchTest/PS_DeathMatch.PS_DeathMatch_C|SetDeath DeadPlayerState (+ (Variables|/Game/Blueprints/DeathMatchTest/PS_DeathMatch.PS_DeathMatch_C|GetDeath DeadPlayerState) 1))
  (if (>= _output_get (Variables|Default|GetWinScore))
    (CallFunction|EndGame)
    (else
      (Utilities|FlowControl|Delay 0.1)
      (CallFunction|OrderPlayerScoreUpdate))))

(event Custom|EndGame
  (for _array_element (Variables|Default|GetPlayerControllerArray)
    (Default|OnGameEnd _array_element))
  (Utilities|FlowControl|Delay 5.0)
  (for _array_element_2 (Variables|Default|GetPlayerControllerArray)
    (|DestroySession _array_element_2
      (:OnSuccess
        (Game|OpenLevel(byName) "MainMap")))))

(event EventBeginPlay)

(event EventTick
  (params (DeltaSeconds :type Float%20%28single-precision%29)))

(event EventPostLogin
  (params (NewPlayer :type Player%20Controller%20Object%20Reference))
  (bind _aspc_death_match (Utilities|Casting|CastToPC_DeathMatch NewPlayer))
  (bind _returnvalue (Utilities|Array|Add (Variables|Default|GetPlayerControllerArray) _aspc_death_match))
  (Variables|/Game/Blueprints/DeathMatchTest/PC_DeathMatch.PC_DeathMatch_C|SetPlayerControllerIndex _aspc_death_match _returnvalue)
  (Variables|/Game/Blueprints/DeathMatchTest/PC_DeathMatch.PC_DeathMatch_C|SetPlayerControllerStateMachine _aspc_death_match "NewEnumerator1"))

(fn ConstructionScript)