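; Player controller for the deathmatch mode, handling login handshake, spawn requests, spider death and player UI.
; A RepNotify state machine drives startup: the local client creates the round widget and sends its GameInstance loadout, then the server stores it and requests a spawn from GM_DeathMatch.
; Deaths report the killer to the game mode and respawn after a delay.
; It also manages the pilot HUD, Tab scoreboard and movement locking.
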(event Custom|ServerRecieveLocalSetting
  (params (UserID :type String) (UserFreeSet :type User%20Free%20Set%20Structure))
  (Networking|SwitchHasAuthority
    (:Authority
      (bind _asps_death_match (Utilities|Casting|CastToPS_DeathMatch (Variables|GetPlayerState)))
      (Variables|/Game/Blueprints/DeathMatchTest/PS_DeathMatch.PS_DeathMatch_C|SetUserID _asps_death_match UserID)
      (Variables|Default|SetCurrentFreeSet UserFreeSet)
      (Variables|Default|SetPlayerControllerStateMachine "NewEnumerator2")
      (Utilities|FlowControl|Delay 0.1)
      (bind _asgm_death_match (Utilities|Casting|CastToGM_DeathMatch (Game|GetGameMode)))
      (Default|OrderPlayerListUpdate _asgm_death_match))))

(event Custom|ClientSendLocalSetting
  (bind _asgi_proto (Utilities|Casting|CastToGI_Proto (Game|GetGameInstance)))
  (CallFunction|ServerRecieveLocalSetting "DefaultID" (Utilities|Array|Get(acopy) (Variables|/Script/Proto.GI_Proto|GetUserFreeSetArray _asgi_proto) (Variables|/Script/Proto.GI_Proto|GetUserFreeSetSelector _asgi_proto))))

(event Custom|AllowMovement
  (Input|ResetIgnoreMoveInput))

(event Custom|ForceStopMovement
  (Input|SetIgnoreMoveInput true))

(event Custom|OnGameEnd
  (Input|SetIgnoreMoveInput self true)
  (Default|ShowScoreBoard (Variables|Default|GetRoundWidget) true))

(event Custom|SendSpawnOrder
  (bind _asgm_death_match (Utilities|Casting|CastToGM_DeathMatch (Game|GetGameMode)))
  (Default|RecieveSpawnOrder _asgm_death_match self (Variables|Default|GetCurrentFreeSet)))

(event Custom|Local%20PostLogin
  (if (Pawn|IsLocalPlayerController)
    (Viewport|RemoveAllWidgets)
    (bind _returnvalue (UserInterface|CreateWidget "/Game/Blueprints/Widget/InBattle/DeathMatch/UMG_DeathMatchRound.UMG_DeathMatchRound_C" self))
    (bind _output_get (Variables|Default|SetRoundWidget _returnvalue))
    (UserInterface|Viewport|AddtoViewport _output_get 10)
    (CallFunction|ClientSendLocalSetting)))

(event Custom|CreatePilotHUDWidget
  (params (WeaponControlSystem :type Weapon%20Control%20System%20Object%20Reference) (DamageControlSystem :type Damage%20Control%20System%20Object%20Reference) (ClassName :type Name))
  (bind _returnvalue (UserInterface|CreateWidget "/Game/Blueprints/Widget/InBattle/UMG_Pilot.UMG_Pilot_C" self))
  (Variables|Default|SetHUDWidget _returnvalue)
  (UserInterface|Viewport|AddtoViewport _returnvalue 1))

(event Custom|OnspiderDeath
  (params (Killer%20Player%20State :type PS%20Death%20Match%20Object%20Reference))
  (CallFunction|LocalonSpiderDeath Killer%20Player%20State)
  (bind _asgm_death_match (Utilities|Casting|CastToGM_DeathMatch (Game|GetGameMode)))
  (bind _asps_death_match (Utilities|Casting|CastToPS_DeathMatch (Variables|GetPlayerState)))
  (Default|GetKillReport _asgm_death_match Killer%20Player%20State _asps_death_match)
  (Utilities|FlowControl|Delay 5.0)
  (Default|RecieveSpawnOrder _asgm_death_match self (Variables|Default|GetCurrentFreeSet)))

(event Custom|Local%20On%20UnPossess
  (Utilities|IsValid (Variables|Default|GetHUDWidget)
    (:Is%20Valid
      (Widget|RemovefromParent (Variables|Default|GetHUDWidget))
      (Variables|Default|SetHUDWidget 0))))

(event Custom|LocalOnSpiderDeath
  (params (KillerPlayerState :type PS%20Death%20Match%20Object%20Reference))
  (if (Pawn|IsLocalPlayerController)
    (Widget|RemovefromParent (Variables|Default|GetHUDWidget))
    (Utilities|IsValid KillerPlayerState
      (:Is%20Valid
        (Development|PrintString (Utilities|String|Append "You Have Been Killed By : " (Variables|/Game/Blueprints/DeathMatchTest/PS_DeathMatch.PS_DeathMatch_C|GetUserID KillerPlayerState)) true false "(R=1.000000,G=0.000000,B=0.833106,A=1.000000)" 2e+01))
      (:Is%20Not%20Valid
        (Development|PrintString "You Have Benn Killed By Unknown" true false "(R=1.000000,G=0.000000,B=0.833106,A=1.000000)" 2e+01)))))

(event Custom|OnResetPlayerList
  (bind _roundwidget (Variables|Default|GetRoundWidget))
  (bind _umg_deathmatchscoreboard (Variables|/Game/Blueprints/Widget/InBattle/DeathMatch/UMG_DeathMatchRound.UMG_DeathMatchRound_C|GetUMG_DeathMatchScoreBoard _roundwidget))
  (Utilities|IsValid _roundwidget
    (:Is%20Valid
      (Utilities|IsValid _umg_deathmatchscoreboard
        (:Is%20Valid
          (Default|ResetPlayerList _umg_deathmatchscoreboard))))))

(event Custom|OnRearrangeScoreBoard
  (bind _roundwidget (Variables|Default|GetRoundWidget))
  (bind _umg_deathmatchscoreboard (Variables|/Game/Blueprints/Widget/InBattle/DeathMatch/UMG_DeathMatchRound.UMG_DeathMatchRound_C|GetUMG_DeathMatchScoreBoard _roundwidget))
  (Utilities|IsValid _roundwidget
    (:Is%20Valid
      (Utilities|IsValid _umg_deathmatchscoreboard
        (:Is%20Valid
          (Default|RearrangePlayerScore _umg_deathmatchscoreboard))))))

(event EventBeginPlay
  (if (Pawn|IsLocalPlayerController)
    (Input|SetInputModeGameOnly self)))

(event EventTick
  (params (DeltaSeconds :type Float%20%28single-precision%29)))

(event EventPossess
  (params (PossessedPawn :type Pawn%20Object%20Reference))
  (bind _asbasic_spider (Utilities|Casting|CastToBasicSpider PossessedPawn))
  (Variables|Default|SetControllingSpider _asbasic_spider))

(event EventUnPossess
  (params (UnpossessedPawn :type Pawn%20Object%20Reference))
  (Variables|Default|SetControllingSpider 0)
  (CallFunction|LocalonUnPossess))

(event Input|KeyboardEvents|Tab
  (params (Key :type Key%20Structure :default "None"))
  (bind _roundwidget (Variables|Default|GetRoundWidget))
  (bind _roundwidget_2 (Variables|Default|GetRoundWidget))
  (:Pressed
    (Utilities|IsValid _roundwidget_2
      (:Is%20Valid
        (Default|ShowScoreBoard _roundwidget_2 true))))
  (:Released
    (Utilities|IsValid _roundwidget
      (:Is%20Valid
        (Default|ShowScoreBoard _roundwidget false)))))

(fn ConstructionScript)

(fn OnRepPlayerControllerStateMachine
  (switch Utilities|FlowControl|Switch|SwitchonBPPlayerControllerState (Variables|Default|GetPlayerControllerStateMachine)
    (:NewEnumerator1
      (if (Pawn|IsLocalPlayerController)
        (CallFunction|LocalPostLogin)))
    (:NewEnumerator2
      (Networking|SwitchHasAuthority
        (:Authority
          (CallFunction|SendSpawnOrder))))))