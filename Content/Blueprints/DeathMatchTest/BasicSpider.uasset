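; BasicSpider is a deathmatch spider pawn that carries two weapons and is possessed by a PC_DeathMatch controller.
; A server-driven state machine waits for client BeginPlay reports (or a fallback timer) and possession, then spawns and syncs weapons on arrow sockets.
; RepNotifies on controller and state create the local pilot HUD.
; Death disables tick, reports the killer, unpossesses, and destroys weapons and pawn after a short delay.
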(event Custom|OnClientBeginPlay
  (bind _output_get (Variables|Default|SetReplicationReady (+ (Variables|Default|GetReplicationReady) 1)))
  (if (>= _output_get (Utilities|Array|Length (Variables|/Script/Engine.GameStateBase|GetPlayerArray (Game|GetGameState))))
    (Variables|Default|SetPawnStateMachine "NewEnumerator2")
    (CallFunction|CheckReadytoAttachWeapon)))

(event Custom|LocalPossessed
  (bind _possessedprotocontroller (Variables|Default|GetPossessedProtoController))
  (if (Pawn|IsLocalPlayerController _possessedprotocontroller)
    (Default|CreatePilotHUDWidget _possessedprotocontroller (Variables|Default|GetWeaponControlSystem) (Variables|Default|GetDamageControlSystem) (Variables|Default|GetClassName))
    (CallFunction|CheckReadytoAttachWeapon)))

(event Custom|CheckReadytoAttachWeapon
  (bind _spawnfailtimehandle (Variables|Default|GetSpawnFailTimeHandle))
  (Networking|SwitchHasAuthority
    (:Authority
      (if (and (Utilities|Enum|Equal(Enum) (Variables|Default|GetPawnStateMachine) "NewEnumerator2") (Variables|Default|GetbIsPossessed))
        (if (Utilities|Time|IsTimerActivebyHandle _spawnfailtimehandle)
          (Utilities|Time|ClearandInvalidateTimerbyHandle _spawnfailtimehandle))
        (Variables|Default|SetPawnStateMachine "NewEnumerator3")
        (CallFunction|SpawnandSyncWeapons)))))

(event Custom|OnFailToRecieveClientBeginPlay
  (Networking|SwitchHasAuthority
    (:Authority
      (Development|PrintString "Fail to check all clients actor replication. Automatically moves to next state" true true "(R=1.000000,G=0.000000,B=0.000000,A=1.000000)" 2e+01)
      (if (<= (Variables|Default|GetPawnStateMachine) 1)
        (Variables|Default|SetPawnStateMachine "NewEnumerator2")
        (CallFunction|CheckReadytoAttachWeapon)
        (else
          (Development|PrintString "WTF!" true true "(R=1.000000,G=0.000000,B=0.000000,A=1.000000)" 2e+01))))))

(event Custom|SpawnAndSyncWeapons
  (bind _arrow1 (Variables|Default|GetArrow1))
  (bind _arrow2 (Variables|Default|GetArrow2))
  (bind _possessedprotocontroller (Variables|Default|GetPossessedProtoController))
  (bind _returnvalue (Transformation|GetWorldTransform _arrow2))
  (bind _returnvalue_2 (Transformation|GetWorldTransform _arrow1))
  (bind _currentfreeset (Variables|/Game/Blueprints/DeathMatchTest/PC_DeathMatch.PC_DeathMatch_C|GetCurrentFreeSet _possessedprotocontroller))
  (Networking|SwitchHasAuthority
    (:Authority
      (Development|PrintString (Utilities|String|BuildString(Integer) "Current Weapon 1 Class" "(" (Utilities|Array|Get(acopy) (.weapon1 _currentfreeset)) ")") true true "(R=1.000000,G=0.000000,B=0.000000,A=1.000000)" 2e+01)
      (bind _returnvalue_3 (Class|BPFSpawnFactory|SpawnWeapon 0 (.location _returnvalue_2) (.rotation _returnvalue_2) self))
      (bind _returnvalue_4 (Class|WeaponControlSystem|SyncNewWeapon (Variables|Default|GetWeaponControlSystem) _returnvalue_3))
      (Development|PrintString (Class|KismetStringLibrary|BuildStringBool "Weapon Sync Result : " "" _returnvalue_4) true true "(R=1.000000,G=0.000000,B=0.000000,A=1.000000)" 2e+01)
      (Development|PrintString (Utilities|String|BuildString(Integer) "Current Weapon 2 Class" "(" (Utilities|Array|Get(acopy) (.weapon2 _currentfreeset)) ")") true true "(R=1.000000,G=0.000000,B=0.000000,A=1.000000)" 2e+01)
      (bind _returnvalue_5 (Class|BPFSpawnFactory|SpawnWeapon 0 (.location _returnvalue) (.rotation _returnvalue) self))
      (bind _returnvalue_6 (Class|WeaponControlSystem|SyncNewWeapon (Variables|Default|GetWeaponControlSystem) _returnvalue_5 1))
      (Development|PrintString (Class|KismetStringLibrary|BuildStringBool "Weapon Sync Result : " "" _returnvalue_6) true true "(R=1.000000,G=0.000000,B=0.000000,A=1.000000)" 2e+01)
      (Variables|Default|SetPawnStateMachine "NewEnumerator4"))))

(event Custom|OnDeath_Event_0
  (params (EventInstigator :type Controller%20Object%20Reference))
  (bind _returnvalue (Pawn|GetController))
  (CallFunction|MulticastActorTickEnabled false)
  (Utilities|IsValid (Variables|Default|GetPossessedProtoController)
    (:Is%20Valid
      (bind _asps_death_match (Utilities|Casting|CastToPS_DeathMatch (Variables|/Script/Engine.Controller|GetPlayerState EventInstigator))
        (:then
          (Default|OnspiderDeath (Variables|Default|GetPossessedProtoController) _asps_death_match))
        (:CastFailed
          (Default|OnspiderDeath (Variables|Default|GetPossessedProtoController)))))
    (:Is%20Not%20Valid
      _))
  (Utilities|Time|SetTimerbyEvent (delegate Custom|DestroyWeaponAndSelf) 0.5)
  (Utilities|IsValid (Variables|Default|GetPossessedProtoController)
    (:Is%20Valid
      (Pawn|UnPossess (Variables|Default|GetPossessedProtoController)))
    (:Is%20Not%20Valid
      (Utilities|IsValid _returnvalue
        (:Is%20Valid
          (Pawn|UnPossess _returnvalue))
        (:Is%20Not%20Valid
          _))))
  (Variables|Default|SetPossessedProtoController 0))

(event Custom|DestroyWeaponAndSelf
  (for _array_element (Variables|/Script/Proto.WeaponControlSystem|GetWeaponDataArray (Variables|Default|GetWeaponControlSystem))
    (Utilities|IsValid (.Weapon (Utilities|Struct|BreakWeaponData _array_element))
      (:Is%20Valid
        (Actor|DestroyActor (.Weapon (Utilities|Struct|BreakWeaponData _array_element))))))
  (Actor|DestroyActor))

(event Custom|MulticastActorTickEnabled
  (params (Enabled :type Boolean))
  (Actor|Tick|SetActorTickEnabled Enabled))

(event EventBeginPlay
  (Class|ChSpiderBase|SetWaistSceneComponent (Variables|Default|GetScene))
  (Networking|SwitchHasAuthority
    (:Authority
      (Class|WeaponControlSystem|SetWeaponSocket (Variables|Default|GetWeaponControlSystem) (Variables|Default|GetArrow1) 0 (Utilities|Array|MakeArray -2e+01 4e+01) (Utilities|Array|MakeArray -1e+01 1e+01))
      (Class|WeaponControlSystem|SetWeaponSocket (Variables|Default|GetWeaponControlSystem) (Variables|Default|GetArrow2) 1 (Utilities|Array|MakeArray -2e+01 4e+01) (Utilities|Array|MakeArray -1e+01 1e+01))
      (EventDispatchers|AssignOnDeath (delegate Custom|OnDeath_Event_0))
      (Variables|Default|SetPawnStateMachine "NewEnumerator1")
      (bind _returnvalue (Utilities|Time|SetTimerbyEvent (delegate Custom|OnFailToRecieveClientBeginPlay) 1.0 false 1.0))
      (Variables|Default|SetSpawnFailTimeHandle _returnvalue))
    (:Remote
      _))
  (CallFunction|OnClientBeginPlay))

(event Collision|EventActorBeginOverlap
  (params (OtherActor :type Actor%20Object%20Reference)))

(event EventTick
  (params (DeltaSeconds :type Float%20%28single-precision%29)))

(event EventPossessed
  (params (NewController :type Controller%20Object%20Reference))
  (Variables|Default|SetbIsPossessed true)
  (bind _aspc_death_match (Utilities|Casting|CastToPC_DeathMatch NewController))
  (Variables|Default|SetPossessedProtoController _aspc_death_match))

(fn ConstructionScript)

(fn OnRepPossessedProtoController
  (bind _possessedprotocontroller (Variables|Default|GetPossessedProtoController))
  (Utilities|IsValid _possessedprotocontroller
    (:Is%20Valid
      (if (Pawn|IsLocalPlayerController _possessedprotocontroller)
        (CallFunction|LocalPossessed)))))

(fn OnRepPawnStateMachine
  (bind _possessedprotocontroller (Variables|Default|GetPossessedProtoController))
  (switch Utilities|FlowControl|Switch|SwitchonBPPawnState (Variables|Default|GetPawnStateMachine)
    (:NewEnumerator4
      (Utilities|IsValid _possessedprotocontroller
        (:Is%20Valid
          (if (Pawn|IsLocalPlayerController _possessedprotocontroller)
            (Default|CreatePilotHUDWidget _possessedprotocontroller (Variables|Default|GetWeaponControlSystem) (Variables|Default|GetDamageControlSystem) "None")))))))