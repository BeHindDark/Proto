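; Deathmatch player controller that handles post-login setup, spawn requests and test HUD widgets for spider pawns.
; A RepNotify state machine triggers local login, which sends the selected free set from GI_Proto to the server.
; The server stores it, sets ReadytoStart and asks GM_DeathMatch to spawn.
; Spider death prints the killer locally and requests a respawn after a delay, while unpossessing clears the controlled spider and pilot HUD.
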(event Custom|ServerRecieveLocalSetting
  (params (UserID :type String) (UserFreeSet :type User%20Free%20Set%20Structure))
  (Networking|SwitchHasAuthority
    (:Authority
      (bind _asps_death_match (Utilities|Casting|CastToPS_DeathMatch (Variables|GetPlayerState))
        (:then
          (Variables|/Game/Blueprints/DebuggingTest/PS_DeathMatch.PS_DeathMatch_C|SetUserID _asps_death_match UserID)
          (Variables|Default|SetCurrentFreeSet UserFreeSet)
          (Variables|Default|SetPlayerControllerStateMachine "NewEnumerator2"))
        (:CastFailed
          (Development|PrintString "WTF3" true true "(R=1.000000,G=0.000000,B=0.000000,A=1.000000)" 2e+01))))))

(event Custom|ClientSendLocalSetting
  (bind _asgi_proto (Utilities|Casting|CastToGI_Proto (Game|GetGameInstance))
    (:then
      (CallFunction|ServerRecieveLocalSetting "DefaultID" (Utilities|Array|Get(acopy) (Variables|/Script/Proto.GI_Proto|GetUserFreeSetArray _asgi_proto) (Variables|/Script/Proto.GI_Proto|GetUserFreeSetSelector _asgi_proto))))
    (:CastFailed
      (Development|PrintString "WTF2" true true "(R=1.000000,G=0.000000,B=0.000000,A=1.000000)" 2e+01))))

(event Custom|SendSpawnOrder
  (bind _asgm_death_match (Utilities|Casting|CastToGM_DeathMatch (Game|GetGameMode)))
  (Default|RecieveSpawnOrder _asgm_death_match self (Variables|Default|GetCurrentFreeSet)))

(event Custom|Local%20PostLogin
  (if (Pawn|IsLocalPlayerController)
    (Viewport|RemoveAllWidgets)
    (bind _returnvalue (UserInterface|CreateWidget "/Game/Blueprints/DebuggingTest/UMG_TestWidget.UMG_TestWidget_C" self true)) ; round widget
    (UserInterface|Viewport|AddtoViewport _returnvalue 0)
    (CallFunction|ClientSendLocalSetting)))

(event Custom|CreatePilotHUDWidget
  (params (WeaponControlSystem :type Weapon%20Control%20System%20Object%20Reference))
  (bind _returnvalue (UserInterface|CreateWidget "/Game/Blueprints/DebuggingTest/UMG_TestWidget.UMG_TestWidget_C" self))
  (UserInterface|Viewport|AddtoViewport _returnvalue 0)
  (Variables|Default|Sethud%20test _returnvalue))

(event Custom|OnspiderDeath
  (params (Killer%20Player%20State :type PS%20Death%20Match%20Object%20Reference))
  (CallFunction|LocalonSpiderDeath Killer%20Player%20State)
  (Utilities|FlowControl|Delay 5.0)
  (bind _asgm_death_match (Utilities|Casting|CastToGM_DeathMatch (Game|GetGameMode)))
  (Default|RecieveSpawnOrder _asgm_death_match self (Variables|Default|GetCurrentFreeSet)))

(event Custom|Local%20On%20UnPossess
  (Utilities|IsValid (Variables|Default|Gethud%20test)
    (:Is%20Valid
      (Widget|RemovefromParent (Variables|Default|Gethud%20test))
      (Variables|Default|Sethud%20test 0))))

(event Custom|LocalOnSpiderDeath
  (params (KillerPlayerState :type PS%20Death%20Match%20Object%20Reference))
  (if (Pawn|IsLocalPlayerController)
    (Utilities|IsValid KillerPlayerState
      (:Is%20Valid
        (Development|PrintString (Utilities|String|Append "You Have Been Killed By : " (Variables|/Game/Blueprints/DebuggingTest/PS_DeathMatch.PS_DeathMatch_C|GetUserID KillerPlayerState)) true false "(R=1.000000,G=0.000000,B=0.833106,A=1.000000)" 2e+01))
      (:Is%20Not%20Valid
        (Development|PrintString "You Have Benn Killed By Unknown" true false "(R=1.000000,G=0.000000,B=0.833106,A=1.000000)" 2e+01)))))

(event EventBeginPlay)

(event EventTick
  (params (DeltaSeconds :type Float%20%28single-precision%29)))

(event EventPossess
  (params (PossessedPawn :type Pawn%20Object%20Reference))
  (bind _asbasic_spider (Utilities|Casting|CastToBasicSpider PossessedPawn))
  (Variables|Default|SetControllingSpider _asbasic_spider))

(event EventUnPossess
  (params (UnpossessedPawn :type Pawn%20Object%20Reference))
  (Variables|Default|SetControllingSpider 0)
  (CallFunction|LocalonUnPossess))

(fn ConstructionScript)

(fn OnRepPlayerControllerStateMachine
  (switch Utilities|FlowControl|Switch|SwitchonBPPlayerControllerState (Variables|Default|GetPlayerControllerStateMachine)
    (:NewEnumerator1
      (if (Pawn|IsLocalPlayerController)
        (CallFunction|LocalPostLogin)))
    (:NewEnumerator2
      (Networking|SwitchHasAuthority
        (:Authority
          (CallFunction|SendSpawnOrder))))))