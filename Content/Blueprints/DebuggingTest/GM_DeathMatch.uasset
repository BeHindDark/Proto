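; GM_DeathMatch is a deathmatch game mode that registers joining players and spawns their pawns.
; PostLogin adds each PC_DeathMatch controller to an array, stores its index on it and sets its state machine value.
; RecieveSpawnOrder unpossesses any current pawn without destroying it, then spawns and possesses a BasicSpider at a player start.
; The UserFreeSet input to that spawn event is unused.
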(event Custom|RecieveSpawnOrder
  (params (PlayerController :type Player%20Controller%20Object%20Reference) (UserFreeSet :type User%20Free%20Set%20Structure))
  (Utilities|IsValid (Pawn|GetControlledPawn PlayerController)
    (:Is%20Valid
      (Pawn|UnPossess PlayerController))
    (:Is%20Not%20Valid
      _))
  (bind _aspc_death_match (Utilities|Casting|CastToPC_DeathMatch PlayerController))
  (bind _returnvalue (Game|SpawnActorfromClass "/Game/Blueprints/DebuggingTest/BasicSpider.BasicSpider_C" (Math|Transform|MakeTransform (.location (Transformation|GetActorTransform (Class|GameModeBase|FindPlayerStart _aspc_death_match))) (.rotation (Transformation|GetActorTransform (Class|GameModeBase|FindPlayerStart _aspc_death_match))) "1,1,1") "AdjustIfPossibleButAlwaysSpawn" _aspc_death_match 0))
  (Pawn|Possess _aspc_death_match _returnvalue))

(event EventBeginPlay)

(event EventTick
  (params (DeltaSeconds :type Float%20%28single-precision%29)))

(event EventPostLogin
  (params (NewPlayer :type Player%20Controller%20Object%20Reference))
  (bind _aspc_death_match (Utilities|Casting|CastToPC_DeathMatch NewPlayer))
  (bind _returnvalue (Utilities|Array|Add (Variables|Default|GetPlayerControllerArray) _aspc_death_match))
  (Variables|/Game/Blueprints/DebuggingTest/PC_DeathMatch.PC_DeathMatch_C|SetPlayerControllerIndex _aspc_death_match _returnvalue)
  (Variables|/Game/Blueprints/DebuggingTest/PC_DeathMatch.PC_DeathMatch_C|SetPlayerControllerStateMachine _aspc_death_match "NewEnumerator1"))

(fn ConstructionScript)