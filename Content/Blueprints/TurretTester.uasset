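; Test actor that exercises the WeaponControlSystem component as a single-weapon turret.
; On BeginPlay it initializes one weapon slot and registers Arrow1 as a socket with yaw and pitch limits.
; It then spawns a ProjectileTest weapon, syncs it to the system and sets a distant world target along +X from the arrow.
; Print strings report success or which setup step failed.
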(event EventBeginPlay
  (Class|WeaponControlSystem|InitializeWeaponNumber (Variables|Default|GetWeaponControlSystem) 1)
  (bind _returnvalue (Class|WeaponControlSystem|SetWeaponSocket (Variables|Default|GetWeaponControlSystem) (Variables|Default|GetArrow1) 0 (Utilities|Array|MakeArray -9e+01 9e+01) (Utilities|Array|MakeArray -9e+01 9e+01)))
  (if _returnvalue
    (bind _returnvalue_2 (Game|SpawnActorfromClass "/Game/Blueprints/ProjectileTest.ProjectileTest_C" (Math|Transform|MakeTransform "0, 0, 0" "0, 0, 0" "1,1,1") "AdjustIfPossibleButAlwaysSpawn" self 0))
    (bind _returnvalue_3 (Class|WeaponControlSystem|SyncNewWeapon (Variables|Default|GetWeaponControlSystem) _returnvalue_2))
    (if _returnvalue_3
      (Development|PrintString "Hello")
      (Variables|/Script/Proto.WeaponControlSystem|SetTargetWorldLocation (Variables|Default|GetWeaponControlSystem) (+ (Transformation|GetWorldLocation (Variables|Default|GetArrow1)) "300000.000000, 0, 0"))
      (else
        (Development|PrintString "Fail2")))
    (else
      (Development|PrintString "Fail1"))))

(event Collision|EventActorBeginOverlap
  (params (OtherActor :type Actor%20Object%20Reference)))

(event EventTick
  (params (DeltaSeconds :type Float%20%28single-precision%29)))

(fn ConstructionScript
  (|CallParentFunction))