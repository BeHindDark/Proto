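; TestSpider is a test spider actor that arms itself with two projectile weapons on BeginPlay.
; It sets its waist scene component, then registers two arrow-based weapon sockets on the WCS with matching yaw and pitch limits.
; If both sockets succeed, the authority spawns the weapons and syncs each into its own index and group, creating the second only after the first syncs.
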(event EventBeginPlay
  (Class|ChSpiderBase|SetWaistSceneComponent (Variables|Default|GetScene))
  (bind _returnvalue (Class|WeaponControlSystem|SetWeaponSocket (Variables|Default|GetWCS) (Variables|Default|GetArrow1) 0 (Utilities|Array|MakeArray -6e+01 6e+01) (Utilities|Array|MakeArray -1e+01 2e+01)))
  (if _returnvalue
    (bind _returnvalue_2 (Class|WeaponControlSystem|SetWeaponSocket (Variables|Default|GetWCS) (Variables|Default|GetArrow2) 1 (Utilities|Array|MakeArray -6e+01 6e+01) (Utilities|Array|MakeArray -1e+01 2e+01)))
    (if _returnvalue_2
      (Networking|SwitchHasAuthority
        (:Authority
          (bind _returnvalue_3 (Game|SpawnActorfromClass "/Game/Blueprints/BP_Act_DB_ProjectileWeaponBase.BP_Act_DB_ProjectileWeaponBase_C" (Math|Transform|MakeTransform "0, 0, 0" "0, 0, 0" "1,1,1") "Undefined" self 0))
          (bind _returnvalue_4 (Class|WeaponControlSystem|SyncNewWeapon (Variables|Default|GetWCS) _returnvalue_3))
          (if _returnvalue_4
            (bind _returnvalue_5 (Game|SpawnActorfromClass "/Game/Blueprints/BP_Act_DB_ProjectileWeaponBase.BP_Act_DB_ProjectileWeaponBase_C" (Math|Transform|MakeTransform "0, 0, 0" "0, 0, 0" "1,1,1") "Undefined" self 0))
            (Class|WeaponControlSystem|SyncNewWeapon (Variables|Default|GetWCS) _returnvalue_5 1 1)))))))

(event Collision|EventActorBeginOverlap
  (params (OtherActor :type Actor%20Object%20Reference)))

(event EventTick
  (params (DeltaSeconds :type Float%20%28single-precision%29)))

(fn ConstructionScript)